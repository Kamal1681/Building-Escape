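; A door actor that swings open and closed in response to OpenDoor's OnOpen and OnClose events.
; It stores its starting rotation at BeginPlay, then a timeline's DoorSwing track adds a yaw offset to that rotation.
; Opening plays the timeline and closing reverses it, so both share one swing curve.
; A door lock sound node is present but disconnected, so it never plays.
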(event `self.ReceiveBeginPlay`
  (set `self.Initial Rotation` (`self.K2_GetActorRotation`)))

(event `self.OpenDoor.OnOpen`
  (bind (_direction _door_swing) (`Timeline|Timeline_0` :!label _label)
    (:`Update`
      (`self.K2_SetActorRotation` (`KismetMathLibrary.ComposeRotators` (`self.Initial Rotation`) (`KismetMathLibrary.MakeRotator` 0.0 0.0 _door_swing))))))

(event `self.OpenDoor.OnClose`
  (goto _label :!via `Reverse`))

(fn `UserConstructionScript`)